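; Game mode for a colour pickup game that creates the information HUD and shows pickup counts on it.
; On BeginPlay it adds the HUD widget, then writes the number of Pickup actors in the level and the red, green and blue progress.
; Each colour's total is derived at runtime as the PickupSpawner count divided by three, assuming equal spawners per type.
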(event `self.ReceiveBeginPlay`
  ;[1 1 1] Add hud
  (bind _returnvalue (`|CreateWidget` "/Game/Blueprints/HUD/InformationHud.InformationHud_C"))
  (bind _output_get (set `self.HUD` _returnvalue))
  (`UserWidget.AddToViewport` _output_get 0)
  (`self.CountRemaining`)
  (`self.UpdateColorProgress`))

(event `self.ReceiveTick`
  (params (DeltaSeconds :type "Float (single-precision)"))
  (switch `/Game/Blueprints/GameMode/GameState` "NewEnumerator0"))

(fn `CountRemaining`
  (bind _outactors (`GameplayStatics.GetAllActorsOfClass` "/Game/Blueprints/PickupSystems/Pickup.Pickup_C"))
  (`TextBlock.SetText` (`/Game/Blueprints/HUD/InformationHud.PickupCount` (`self.HUD`)) (`KismetTextLibrary.Conv_IntToText` (`KismetArrayLibrary.Array_Length` _outactors))))

(fn `ProgressFormat`
  (params (ColorProgress :type Integer))
  (returns (FormatCompletion :type Text))
  ;[1 1 1] Amount of spawners divided by 3 types = amount per type
  (bind _outactors (`GameplayStatics.GetAllActorsOfClass` "/Game/Blueprints/PickupSystems/PickupSpawner.PickupSpawner_C"))
  (return (`|FormatText` "{progess}/{total}" ColorProgress (/ (`KismetArrayLibrary.Array_Length` _outactors) 3))))

(fn `UpdateColorProgress`
  (`|ExecutionSequence`
    (:`then_0`
      (bind _formatcompletion (`self.ProgressFormat` (`self.RedProgress`)))
      (`TextBlock.SetText` (`/Game/Blueprints/HUD/InformationHud.RedPickups` (`self.HUD`)) _formatcompletion))
    (:`then_1`
      (bind _formatcompletion_2 (`self.ProgressFormat` (`self.GreenProgress`)))
      (`TextBlock.SetText` (`/Game/Blueprints/HUD/InformationHud.GreenPickups` (`self.HUD`)) _formatcompletion_2))
    (:`then_2`
      (bind _formatcompletion_3 (`self.ProgressFormat` (`self.BlueProgress`)))
      (`TextBlock.SetText` (`/Game/Blueprints/HUD/InformationHud.BluePickups` (`self.HUD`)) _formatcompletion_3))))

(fn `UserConstructionScript`)